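; BP_SwitchActor is a pressure switch that sinks and changes color when something overlaps its box.
; BeginPlay creates a dynamic material instance from the mesh's material and tints it with SwitchColor.
; Overlap plays a timeline that lowers the mesh and blends the tint to blue, then calls TurnedOn or TurnedOff on finish by direction.
; TurnOff, or ending overlap when AutoReturnIsMomentary is set, reverses the timeline.
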(event `self.ReceiveBeginPlay`
  (bind _mesh (`self.Mesh`))
  ;[1 1 1] 밟으면 버튼 색이 변함
  (bind _returnvalue (`PrimitiveComponent.CreateDynamicMaterialInstance` _mesh 0 (`PrimitiveComponent.GetMaterial` _mesh 0) "None"))
  (bind _output_get (set `self.MI_Swtich` _returnvalue))
  (`MaterialInstanceDynamic.SetVectorParameterValue` _output_get "Tint Base Color" (`self.SwitchColor`)))

(event `self.Box.OnComponentBeginOverlap`
  (params (OverlappedComponent :type "PrimitiveComponent Object Reference") (OtherActor :type "Actor Object Reference") (OtherComp :type "PrimitiveComponent Object Reference") (OtherBodyIndex :type Integer) (bFromSweep :type Boolean) (SweepResult :type "HitResult Structure (by ref)"))
  (bind (_direction _alpha) (`Timeline|SwitchTimeLine` :!label _label)
    (:`Update`
      (`SceneComponent.K2_SetRelativeLocation` (`self.Mesh`) (`KismetMathLibrary.VLerp` (0.0 0.0 0.0) (0.0 0.0 -7.0) _alpha) false false)
      (`MaterialInstanceDynamic.SetVectorParameterValue` (`self.MI_Swtich`) "Tint Base Color" (`KismetMathLibrary.LinearColorLerp` (`self.SwitchColor`) (struct :`R` 0.007688 :`B` 1.0 :`A` 1.0) _alpha)))
    (:`Finished`
      (switch `ETimelineDirection` _direction
        (:`Forward`
          (`self.TurnedOn`))
        (:`Backward`
          (`self.TurnedOff`))))))

(event `TurnOff`
  (goto _label :!via `Reverse`))

(event `self.Box.OnComponentEndOverlap`
  (params (OverlappedComponent :type "PrimitiveComponent Object Reference") (OtherActor :type "Actor Object Reference") (OtherComp :type "PrimitiveComponent Object Reference") (OtherBodyIndex :type Integer))
  (if (`self.AutoReturn (IsMomentary)`)
    (goto _label :!via `Reverse`)))

(fn `UserConstructionScript`)