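; Game mode that respawns the player pawn whenever it is destroyed and manages the background music.
; BeginPlay binds the initial pawn's OnDestroyed event, leading to RespawnPlayer, which spawns a BP_PlayerPawn at the player start and possesses it.
; Each new pawn's OnDestroyed is bound again, so respawning repeats indefinitely.
; PlayBGM swaps tracks on a single MusicSpeaker, restarting the music at game start and each respawn.
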(event `self.ReceiveBeginPlay`
  ;[1 1 1] 시작 플레이어 소멸자에 이벤트 연결
  (add `self.OnDestroyed` (`GameplayStatics.GetPlayerPawn` 0) (delegate `RespawnFirst`))
  (`self.PlayBGM` "/Game/Audio/bgm02_Cue.bgm02_Cue"))

(event `RespawnFirst` :!signature `self.OnDestroyed`
  (params (DestroyedActor :type "Actor Object Reference"))
  ;[1 1 1] 시작 플레이어 소멸자에 이벤트 연결
  (`self.RespawnPlayer`))

(event `RespawnPlayer`
  ;[1 1 1] 죽으면 게임 시작위치에서 플레이어 소환하기
  (bind _returnvalue (`|SpawnActorFromClass` "/Game/BluePrints/BP_PlayerPawn.BP_PlayerPawn_C" (`self.GetTransform` (`self.K2_FindPlayerStart` null)) "Undefined" "OverrideRootScale" null null))
  (`Controller.Possess` (`GameplayStatics.GetPlayerController` 0) _returnvalue)
  ;[1 1 1] 새로 생성된 플레이어에도 이벤트 적용
  (add `self.OnDestroyed` _returnvalue (delegate `RespawnRepiter`))
  (`self.PlayBGM` "/Game/Audio/bgm02_Cue.bgm02_Cue"))

(event `RespawnRepiter` :!signature `self.OnDestroyed`
  (params (DestroyedActor :type "Actor Object Reference"))
  ;[1 1 1] 새로 생성된 플레이어에도 이벤트 적용
  (`self.RespawnPlayer`))

(fn `PlayBGM`
  (params (NewBGM :type "SoundCue Object Reference"))
  (bind _musicspeaker (`self.MusicSpeaker`))
  ;[1 1 1] 음악이 하나만 재생되는 베타제어 재생
  (`AudioComponent.Stop` _musicspeaker)
  (`AudioComponent.SetSound` _musicspeaker NewBGM)
  (`AudioComponent.Play` _musicspeaker 0.0))

(fn `UserConstructionScript`)