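; Player character with camera-relative movement, sprint, and a coin count that sprinting puts at risk.
; A looping timer drops a coin at sprint speed, spawning a physics pickup from a mesh socket with a randomly rotated impulse.
; The first damage taken ragdolls the player, spills all coins, blocks further collection and sets a lifespan.
; Death and scroll pickup, which marks the goal and stops movement, each switch BGM through BP_GameMode.
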(event `self.ReceiveBeginPlay`
  (set `self.IsAbleToAddCoins` true)
  (`KismetSystemLibrary.K2_SetTimer` null "CheckSprintRisk" 0.5 true) ; 일정시간마다 속도 확인해서 코인 감소하는 함수호출
)

(event `InputAction|Sprint`
  (params (Key :type "Key Structure"))
  (bind _charactermovement (`self.CharacterMovement`))
  ;[1 1 1] 달리기
  (:`Pressed`
    (set `CharacterMovementComponent.MaxWalkSpeed` (`self.SprintMoveSpeed (Ground Walk Speed)`) _charactermovement))
  (:`Released`
    (set `CharacterMovementComponent.MaxWalkSpeed` (`self.InitMaxMoveSpeed`) _charactermovement)))

(event `InputAxis|MoveForward`
  (params (AxisValue :type "Float (single-precision)"))
  ;[1 1 1] 이동
  (bind _returnvalue (`/Game/BluePrints/BP_FuncLibrary.Flatten Direction_BP` (`SceneComponent.GetForwardVector` (`self.Camera`))))
  (`self.AddMovementInput` _returnvalue AxisValue))

(event `InputAxis|MoveRight`
  (params (AxisValue :type "Float (single-precision)"))
  ;[1 1 1] 이동
  (bind _returnvalue (`/Game/BluePrints/BP_FuncLibrary.Flatten Direction_BP` (`SceneComponent.GetRightVector` (`self.Camera`))))
  (`self.AddMovementInput` _returnvalue AxisValue))

(event `InputAxis|LookUp`
  (params (AxisValue :type "Float (single-precision)"))
  ;[1 1 1] 카메라- SprintArm에서 Use Control Ratation을 체크 시 카메라가 움직임
  (if (`self.IsLookUpReverse`)
    (`self.AddControllerPitchInput` (* -1 AxisValue))
    (else
      (`self.AddControllerPitchInput` AxisValue))))

(event `InputAxis|LookRight`
  (params (AxisValue :type "Float (single-precision)"))
  ;[1 1 1] 카메라- SprintArm에서 Use Control Ratation을 체크 시 카메라가 움직임
  (`self.AddControllerYawInput` AxisValue))

(event `self.ReceiveAnyDamage`
  (params (Damage :type "Float (single-precision)") (DamageType :type "DamageType Object Reference") (InstigatedBy :type "Controller Object Reference") (DamageCauser :type "Actor Object Reference"))
  (bind _mesh (`self.Mesh`))
  ;[1 1 1] 한번 피해 받으면 멈추고 2초뒤 죽음
  (`/Engine/EditorBlueprintResources/StandardMacros.DoOnce` false
    (:`Completed`
      (`|ExecutionSequence`
        (:`then_0`
          (`KismetSystemLibrary.PrintString` "Hit" true true (struct :`G` 0.66 :`B` 1.0 :`A` 1.0) 3.0)
          (`CharacterMovementComponent.DisableMovement` (`self.CharacterMovement`))
          (`self.SetLifeSpan` 3.0) ; 특정 시간뒤 죽음
          (`PrimitiveComponent.SetCollisionProfileName` _mesh "Ragdoll" true) ; 죽을때만 래그돌로 변경
          (`PrimitiveComponent.SetSimulatePhysics` _mesh true) ; Mesh의 콜리전 ragdol 변경- 죽으면 시체가됨 - ragdol의 계산을 줄이기 위해 원복
        )
        (:`then_1`
          (`self.DropAllCoins`)
          (set `self.IsAbleToAddCoins` false)
          (`ActorComponent.Activate` (`self.DeathFX`) false) ; 죽을때 이펙트 동작
          (`GameplayStatics.PlaySoundAtLocation` "/Game/Audio/player_death_Cue.player_death_Cue" (`self.K2_GetActorLocation`) (struct) 1.0 1.0 0.0 null null null)
          (`KismetSystemLibrary.Delay` 0.5)
          (`/Game/BluePrints/BP_GameMode.PlayBGM` (cast `/Game/BluePrints/BP_GameMode` (`GameplayStatics.GetGameMode`) :!pure true) "/Game/Audio/bgm03_Cue.bgm03_Cue"))))))

(event `ObtainScroll`
  ;[1 1 1] 스크롤 획득
  (`CharacterMovementComponent.DisableMovement` (`self.CharacterMovement`))
  (set `self.HasScroll` true)
  (`KismetSystemLibrary.PrintString` "Goal !!")
  (`/Game/BluePrints/BP_GameMode.PlayBGM` (cast `/Game/BluePrints/BP_GameMode` (`GameplayStatics.GetGameMode`) :!pure true) "/Game/Audio/bgm04_Cue.bgm04_Cue")
  (`KismetSystemLibrary.Delay` 5.0))

(event `DropAllCoins`
  ;[1 1 1] 코인 전부 드랍
  (while (> (`self.NumOfCoins`) 0)
    (`self.DropCoin`)))

(fn `AddCoin`
  (params (AddNum :type Integer))
  (returns (IsAbleToAddCoins :type Boolean))
  (if (`self.IsAbleToAddCoins`)
    (bind _output_get (set `self.NumOfCoins` (+ AddNum (`self.NumOfCoins`))))
    (`KismetSystemLibrary.PrintString` (`KismetStringLibrary.Conv_IntToString` _output_get)))
  (return (`self.IsAbleToAddCoins`)))

(fn `CheckSprintRisk`
  (if (>= (`/Game/BluePrints/BP_ActorMacroLibrary.GetflatSpeed`) (`self.SprintMoveSpeed (Ground Walk Speed)`))
    (`KismetSystemLibrary.PrintString` "속도가 너무 빠릅니다")
    (`self.DropCoin`)))

(fn `DropCoin`
  (locals (`Impulse X` :type Integer :default 0) (`Impulse Y` :type Integer :default 0) (NewLocalVar_0 :type Boolean))
  (bind _output_get (set `self.NumOfCoins` (- (`self.NumOfCoins`) 1)))
  (if (< _output_get 0)
    (set `self.NumOfCoins` 0)
    (`KismetSystemLibrary.PrintString` (`KismetStringLibrary.Conv_IntToString` (`self.NumOfCoins`)))
    (else
      (`KismetSystemLibrary.PrintString` (`KismetStringLibrary.Conv_IntToString` (`self.NumOfCoins`)))
      ;[1 1 1] 코인 떨어뜨림 (닌자 스켈레톤의 헤드에 소켓을 새로 만듦)
      (bind _returnvalue (`|SpawnActorFromClass` "/Game/BluePrints/BP_PickUpCoinActor.BP_PickUpCoinActor_C" (`SceneComponent.GetSocketTransform` (`self.Mesh`) "CoinSpawnPoint" "RTS_World") "Undefined" "OverrideRootScale" null null))
      (bind _staticmeshcomponent (`StaticMeshActor.StaticMeshComponent` _returnvalue))
      (`PrimitiveComponent.SetSimulatePhysics` _staticmeshcomponent true)
      (`PrimitiveComponent.AddImpulse` _staticmeshcomponent (`KismetMathLibrary.RotateAngleAxis` (`KismetMathLibrary.MakeVector` 0.0 100.0 200.0) (`KismetMathLibrary.RandomFloatInRange` 0.0 180.0) (0.0 0.0 1.0)) "None" true) ; 힘을 가해서 팅겨나옴
    )))

(fn `GetNunCoins`
  (returns (NewParam :type Integer))
  ;[1 1 1] 함수는 반환이 필요할때 사용 나머지는 이벤트로 만들어서 사용
  (return (`self.NumOfCoins`)))

(fn `UserConstructionScript`
  (set `CharacterMovementComponent.MaxWalkSpeed` (`self.InitMaxMoveSpeed`) (`self.CharacterMovement`)))