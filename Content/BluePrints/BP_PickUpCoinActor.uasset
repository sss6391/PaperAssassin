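; Coin pickup actor that adds one coin to the player pawn when overlapped.
; A timer opens a gate about a second after BeginPlay, so overlaps before then are ignored, while a timeline drives the mesh's yaw spin.
; Gated overlaps cast to BP_PlayerPawn and call AddCoin; on success the coin destroys itself and spawns a pickup particle effect.
; An unconnected tag-based destroy check remains unused.
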(event `self.ReceiveBeginPlay`
  (`KismetSystemLibrary.K2_SetTimer` null "EnablePickup" 1.0) ; 생성후 0.5초뒤 획득 가능
  ;[1 1 1] 코인이 회전하는 모션
  (bind (_direction _coinyaw) (`Timeline|CoinRotationTimeline`)
    (:`Update`
      (`SceneComponent.K2_SetRelativeRotation` (`self.StaticMeshComponent`) (`KismetMathLibrary.MakeRotator` 0.0 0.0 _coinyaw) false false))))

(event `EnablePickup`
  ;[1 1 1] 오버랩시 BP_PlayerPawn 형 변환 및 코인추가, 셀프삭제
  (goto _label :!via `Open`))

(event `self.Box Trigger.OnComponentBeginOverlap`
  (params (OverlappedComponent :type "PrimitiveComponent Object Reference") (OtherActor :type "Actor Object Reference") (OtherComp :type "PrimitiveComponent Object Reference") (OtherBodyIndex :type Integer) (bFromSweep :type Boolean) (SweepResult :type "HitResult Structure (by ref)"))
  ;[1 1 1] 오버랩시 BP_PlayerPawn 형 변환 및 코인추가, 셀프삭제
  (`/Engine/EditorBlueprintResources/StandardMacros.Gate` true :!label _label
    (:`Exit`
      (bind _asbp_player_pawn (cast `/Game/BluePrints/BP_PlayerPawn` OtherActor)) ; 캐스팅에 실패하면 다른 액터에 들어온 것이니 따로 확인 하지 않아도 됨
      (bind _isabletoaddcoins (`/Game/BluePrints/BP_PlayerPawn.AddCoin` _asbp_player_pawn 1))
      (if _isabletoaddcoins
        (`self.K2_DestroyActor`)
        (`GameplayStatics.SpawnEmitterAtLocation` "/Game/Particle/PS_Pickup_Coin.PS_Pickup_Coin" (`self.K2_GetActorLocation`))))))

(fn `UserConstructionScript`)