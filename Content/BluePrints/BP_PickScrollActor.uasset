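; BP_PickScrollActor is a scroll pickup that bobs up and down in the world until the player pawn collects it.
; On BeginPlay it records the root's world location and plays a timeline (위아래로흔들거림, "bobbing up and down") that offsets the actor's Z from that origin.
; When BP_PlayerPawn overlaps the BoxTrigger, it calls ObtainScroll on the pawn and destroys itself.
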(event `self.ReceiveBeginPlay`
  (bind (_returnvalue_x _returnvalue_y _returnvalue_z) (`KismetMathLibrary.BreakVector` (`SceneComponent.K2_GetComponentLocation` (`self.SceneRoot`))))
  (set `self.Return Value X` _returnvalue_x)
  (set `self.Return Value Z` _returnvalue_z)
  (set `self.Return Value Y` _returnvalue_y)
  (bind (_direction `_축`) (`Timeline|위아래로 흔들거림`)
    (:`Update`
      (`self.K2_SetActorLocation` (`KismetMathLibrary.MakeVector` (`self.Return Value X`) (`self.Return Value Y`) (+ `_축` (`self.Return Value Z`)))))))

(event `self.BoxTrigger.OnComponentBeginOverlap`
  (params (OverlappedComponent :type "PrimitiveComponent Object Reference") (OtherActor :type "Actor Object Reference") (OtherComp :type "PrimitiveComponent Object Reference") (OtherBodyIndex :type Integer) (bFromSweep :type Boolean) (SweepResult :type "HitResult Structure (by ref)"))
  (bind _asbp_player_pawn (cast `/Game/BluePrints/BP_PlayerPawn` OtherActor))
  (`/Game/BluePrints/BP_PlayerPawn.ObtainScroll` _asbp_player_pawn)
  (`self.K2_DestroyActor`))

(fn `UserConstructionScript`)