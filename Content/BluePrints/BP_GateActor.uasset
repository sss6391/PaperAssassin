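; BP_GateActor is a sliding gate with Open and Close events that play and reverse one timeline.
; The timeline's vector track moves the left inner mesh, and the same value with Y negated mirrors the right.
; PlaySE sets the Speaker's "SE Type" parameter, called with the direction at the Opening event track and separately when Close starts.
; An earlier two-track timeline version remains disconnected.
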(event `Open`
  ;[1 1 1] 커스텀 이벤트로 문열림
  (bind (_direction `_left_백터_트랙`) (`Timeline|GateTimeline` :!label _label)
    (:`Update`
      (`SceneComponent.K2_SetRelativeLocation` (`self.Inside Left Mesh`) `_left_백터_트랙` false false)
      (`SceneComponent.K2_SetRelativeLocation` (`self.Inside Right Mesh`) (* `_left_백터_트랙` (1.0 -1.0 1.0)) false false))
    (:`Opening이벤트 트랙`
      (`self.PlaySE` (`KismetMathLibrary.Conv_ByteToInt` _direction)) ; 문 닫히는 사운드
    )))

(event `Close`
  ;[1 1 1] 커스텀 이벤트로 문열림
  (`self.PlaySE` 2)
  (goto _label :!via `Reverse`))

(fn `PlaySE`
  (params (PlayType :type Integer))
  (bind _speaker (`self.Speaker`))
  (`AudioComponent.SetIntParameter` _speaker "SE Type" PlayType)
  (`AudioComponent.Play` _speaker 0.0))

(fn `UserConstructionScript`)