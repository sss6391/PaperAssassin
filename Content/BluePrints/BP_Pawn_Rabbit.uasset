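; BP_Pawn_Rabbit is an AI enemy character that sprints and deals damage on contact.
; While sprinting, a short forward trace from the spine socket damages whatever it hits each tick; capsule hits also apply damage.
; CanSeePlayerPawn line-traces forward on a Sight channel for a Player-tagged actor, polled by a behavior tree service per its comment.
; BegineSprint and EndSprint toggle walk speed and the sprint flag.
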(event `self.ReceiveTick`
  (params (DeltaSeconds :type "Float (single-precision)"))
  (bind _returnvalue (`SceneComponent.GetSocketLocation` (`self.Mesh`) "spine"))
  ;[1 1 1] 공격모드_ 더 가까이 가서 죽게만듦
  (if (`self.IsSprint`)
    (bind _outhit (`KismetSystemLibrary.LineTraceSingle` :`Start` _returnvalue :`End` (+ _returnvalue (* (`self.GetActorForwardVector`) 10.0)) :`TraceChannel` "TraceTypeQuery1" :`DrawDebugType` "ForOneFrame"))
    (bind (_bblockinghit _binitialoverlap _time _distance _location _impactpoint _normal _impactnormal _physmat _hitactor) (`GameplayStatics.BreakHitResult` _outhit))
    (if _bblockinghit
      (`GameplayStatics.ApplyDamage` _hitactor 100.0))))

(event `self.CapsuleComponent.OnComponentHit`
  (params (HitComponent :type "PrimitiveComponent Object Reference") (OtherActor :type "Actor Object Reference") (OtherComp :type "PrimitiveComponent Object Reference") (NormalImpulse :type "Vector Structure") (Hit :type "HitResult Structure (by ref)"))
  ;[1 1 1] 부딪히면 그 물체에 데미지를 부여
  (`GameplayStatics.ApplyDamage` OtherActor 100.0))

(fn `BegineSprint`
  (set `CharacterMovementComponent.MaxWalkSpeed` (`self.SprintGroundSpeed`) (`self.CharacterMovement`))
  (set `self.IsSprint` true))

(fn `CanSeePlayerPawn`
  (returns (ReturnValue :type Boolean) (SeenActor :type "Actor Object Reference"))
  (bind _returnvalue (`self.K2_GetActorLocation`))
  ;[1 1 1] 프로젝스 - 콜리젼 -  트레이스에 Sight 추가
  ;[1 1 1] 라인상에 물체가 있는지 확인
  (bind (_outhit _returnvalue_2) (`KismetSystemLibrary.LineTraceSingle` :`Start` _returnvalue :`End` (+ _returnvalue (* (`self.GetActorForwardVector`) (`self.SightLength`))) :`TraceChannel` "TraceTypeQuery3" :`DrawDebugType` "ForOneFrame"))
  (if _returnvalue_2
    (bind (_bblockinghit _binitialoverlap _time _distance _location _impactpoint _normal _impactnormal _physmat _hitactor) (`GameplayStatics.BreakHitResult` _outhit))
    (return (`self.ActorHasTag` _hitactor "Player") _hitactor)))

(fn `EndSprint`
  (set `CharacterMovementComponent.MaxWalkSpeed` (`self.WalkGroundSpeed`) (`self.CharacterMovement`))
  (set `self.IsSprint` false))

(fn `UserConstructionScript`)